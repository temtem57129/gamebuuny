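; BossBP is a boss character that performs a swipe attack and damages the player on contact.
; Attack plays the Orc_Swiping animation, flags the boss as attacking for a timed window, then restores the Animation Blueprint.
; A Punch collision component, attached to the LeftHand socket in the construction script, deals damage to overlapping ThirdPersonCharacter actors only while that flag is set.
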(event `Attack`
  (`SkeletalMeshComponent.PlayAnimation` (`self.Mesh`) "/Game/BunnyProject/Boss/Mesh_and_Animation/Animation/Orc_Swiping.Orc_Swiping" false)
  (set `self.Attacking` true)
  (`KismetSystemLibrary.Delay` 2.6)
  (set `self.Attacking` false)
  (`SkeletalMeshComponent.SetAnimationMode` (`self.Mesh`) "AnimationBlueprint"))

(event `self.punch.OnComponentBeginOverlap`
  (params (OverlappedComponent :type "PrimitiveComponent Object Reference") (OtherActor :type "Actor Object Reference") (OtherComp :type "PrimitiveComponent Object Reference") (OtherBodyIndex :type Integer) (bFromSweep :type Boolean) (SweepResult :type "HitResult Structure (by ref)"))
  (if (`self.Attacking`)
    (bind _asthird_person_character (cast `/Game/ThirdPersonBP/Blueprints/ThirdPersonCharacter` OtherActor))
    (`/Game/ThirdPersonBP/Blueprints/ThirdPersonCharacter.TakeDamage` _asthird_person_character 10)))

(fn `UserConstructionScript`
  (`SceneComponent.K2_AttachToComponent` (`self.punch`) (`self.Mesh`) "LeftHand" "KeepRelative" "KeepRelative" "KeepRelative" true))