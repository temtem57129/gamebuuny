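; Boss_AI is the AI controller that drives the boss pawn.
; On possessing a BossBP it caches the boss and runs the Boss_BT behavior tree.
; Perception updates for the player character write the sensed state to the CanSeePlayer blackboard key.
; An Attack event forwards to the boss's own Attack.
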(event `self.AIPerception.OnTargetPerceptionUpdated`
  (params (Actor :type "Actor Object Reference") (Stimulus :type "AIStimulus Structure"))
  (cast `/Game/ThirdPersonBP/Blueprints/ThirdPersonCharacter` Actor)
  (`BlackboardComponent.SetValueAsBool` (`AIBlueprintHelperLibrary.GetBlackboard` null) "CanSeePlayer" (`.bSuccessfullySensed` (break `AIStimulus` Stimulus))))

(event `self.ReceivePossess`
  (params (PossessedPawn :type "Pawn Object Reference"))
  (bind _asboss_bp (cast `/Game/BunnyProject/Boss/Mesh_and_Animation/Blueprints/BossBP` PossessedPawn))
  (set `self.Boss` _asboss_bp)
  (`self.RunBehaviorTree` "/Game/BunnyProject/Boss/Mesh_and_Animation/Blueprints/Boss_BT.Boss_BT"))

(event `Attack`
  (`/Game/BunnyProject/Boss/Mesh_and_Animation/Blueprints/BossBP.Attack` (`self.Boss`)))

(fn `UserConstructionScript`)